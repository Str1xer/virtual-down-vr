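; BP_Debuger is a debug actor that shows the player character's position and camera position on a TextRender component.
; On BeginPlay it casts player pawn 0 to BP_Character and caches the reference.
; Each Tick it rebuilds the text from the character's actor location and its Camera's world location, without checking that the cached reference is valid.
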(event `self.ReceiveBeginPlay`
  (bind _asbp_character (cast `/Game/Blueprints/Character/BP_Character` (`GameplayStatics.GetPlayerPawn` 0)))
  (set `self.CharacterRef` _asbp_character))

(event `self.ReceiveTick`
  (params (DeltaSeconds :type "Float (single-precision)"))
  (`TextRenderComponent.K2_SetText` (`self.TextRender`) (`KismetTextLibrary.Conv_StringToText` (`KismetStringLibrary.Concat_StrStr` "Actor Location: " (`KismetStringLibrary.Conv_VectorToString` (`self.K2_GetActorLocation` (`self.CharacterRef`))) " \nCamera Location: " (`KismetStringLibrary.Conv_VectorToString` (`SceneComponent.K2_GetComponentLocation` (`/Game/Blueprints/Character/BP_Character.Camera` (`self.CharacterRef`))))))))

(fn `UserConstructionScript`)