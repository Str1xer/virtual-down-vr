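; BP_VRCard is a VR card actor that displays a configurable puzzle image on its plane.
; The construction script feeds PuzzleTexture into a dynamic instance of M_CardObject.
; OnGrip starts a looping timer, presumably for TickPuzzleChecker, which line-traces out from the card border along its negative right vector with debug drawing.
; The trace result is not used yet, and OnUsed is empty.
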(event `VRGripInterface.OnUsed`)

(event `VRGripInterface.OnGrip`
  (params (GrippingController :type "GripMotionControllerComponent Object Reference") (GripInformation :type "BPActorGripInformation Structure (by ref)"))
  (bind _returnvalue (`KismetSystemLibrary.K2_SetTimerDelegate` (`|CreateDelegate` :!event `TickPuzzleChecker`) 0.2 true))
  (set `self.CheckerTimer` _returnvalue))

(fn `TickPuzzleChecker`
  (bind _sm_cardborder (`self.SM_CardBorder`))
  (bind _returnvalue (`SceneComponent.K2_GetComponentLocation` _sm_cardborder))
  (`KismetSystemLibrary.LineTraceSingle` :`Start` _returnvalue :`End` (+ _returnvalue (* (`SceneComponent.GetRightVector` _sm_cardborder) -1000.0)) :`TraceChannel` "TraceTypeQuery1" :`DrawDebugType` "ForDuration"))

(fn `UserConstructionScript`
  (bind _returnvalue (`KismetMaterialLibrary.CreateDynamicMaterialInstance` "/Game/FirstPersonBP/Blueprints/M_CardObject.M_CardObject"))
  (`MaterialInstanceDynamic.SetTextureParameterValue` _returnvalue "Puzzle Image" (`self.PuzzleTexture`))
  (`PrimitiveComponent.SetMaterial` (`self.Plane`) 0 _returnvalue))