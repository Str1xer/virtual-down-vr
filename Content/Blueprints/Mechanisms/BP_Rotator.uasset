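; BP_Rotator is an interactable puzzle mechanism whose cylinder turns through eight color positions in 45-degree steps.
; Components tagged "Interaction" block a custom trace channel and use custom depth stencil values for hover highlighting.
; Interact plays a sound, advances the wrapping color index and animates the turn with a timeline, ignoring input until it finishes.
; CheckIsSolved reports success at either of two opposite positions.
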(event `self.ReceiveBeginPlay`
  (for _array_element (`self.GetComponentsByTag` "/Script/Engine.PrimitiveComponent" "Interaction")
    (`PrimitiveComponent.SetRenderCustomDepth` _array_element true)
    (`PrimitiveComponent.SetCollisionResponseToChannel` _array_element "ECC_GameTraceChannel3" "ECR_Block"))
  (`SceneComponent.K2_SetRelativeRotation` (`self.Cylinder1`) (`KismetMathLibrary.MakeRotator` 0.0 0.0 (* (`self.CurrentColor`) 45.0)) false false))

(event `/Game/BPI_Interaction.Hover`
  (for _array_element (`self.GetComponentsByTag` "/Script/Engine.PrimitiveComponent" "Interaction")
    (`PrimitiveComponent.SetCustomDepthStencilValue` _array_element 1)))

(event `/Game/BPI_Interaction.Unhover`
  (for _array_element (`self.GetComponentsByTag` "/Script/Engine.PrimitiveComponent" "Interaction")
    (`PrimitiveComponent.SetCustomDepthStencilValue` _array_element 0)))

(event `/Game/BPI_Interaction.Interact`
  (params (Player :type "/Game/FirstPersonBP/Blueprints/BP__Player Object Reference"))
  (bind (_currentrotation_roll _currentrotation_pitch _currentrotation_yaw) (`KismetMathLibrary.BreakRotator` (`self.CurrentRotation`)))
  (bind (_returnvalue_location _returnvalue_rotation) (`KismetMathLibrary.BreakTransform` (`SceneComponent.GetRelativeTransform` (`self.Cylinder1`))))
  (bind _returnvalue (+ (`self.CurrentColor`) 1))
  (if (`self.bCanInteract`)
    (`GameplayStatics.PlaySoundAtLocation` "/Game/Sounds/flashlight_on.flashlight_on" (`self.K2_GetActorLocation`) (struct) 1.0 1.0 0.0 null null null)
    (set `self.CurrentColor` (`KismetMathLibrary.SelectInt` 0 _returnvalue (>= _returnvalue 8)))
    (set `self.CurrentRotation` _returnvalue_rotation)
    (set `self.bCanInteract` false)
    (bind (_direction _ratio) (`Timeline|Ratio` :!via `PlayFromStart`)
      (:`Update`
        (`SceneComponent.K2_SetRelativeRotation` (`self.Cylinder1`) (`KismetMathLibrary.MakeRotator` 0.0 0.0 (+ (* _ratio 45.0) _currentrotation_yaw)) false false))
      (:`Finished`
        (set `self.bCanInteract` true)))))

(fn `CheckIsSolved`
  (returns (State :type Boolean))
  (return (or (== (`self.CurrentColor`) 0) (== (`self.CurrentColor`) 4))))

(fn `UserConstructionScript`)