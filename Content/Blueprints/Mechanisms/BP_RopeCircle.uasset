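; BP_RopeCircle is a mechanism actor with an inner cylinder that can be recolored and moved along its local Z axis in steps.
; ChangeColor swaps the cylinder's material.
; Open plays the ChangeLength timeline, teleporting the cylinder by a scaled curve offset from a fixed base height.
; A step counter increments when the timeline finishes, so each Open continues from the previous stop.
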(event `self.ReceiveBeginPlay`)

(event `/Game/BPI_Door.ChangeColor`
  (params (`New Material` :type "MaterialInstance Object Reference"))
  (`PrimitiveComponent.SetMaterial` (`self.circleInner_Cylinder_001`) 0 `New Material`))

(event `/Game/BPI_Door.Open`
  (bind _targetoffset (`self.TargetOffset`))
  (bind (_direction _z_offset) (`Timeline|ChangeLength` :!via `PlayFromStart`)
    (:`Update`
      (`SceneComponent.K2_SetRelativeLocation` (`self.circleInner_Cylinder_001`) (`KismetMathLibrary.MakeVector` 0.0 0.0 (+ (* _z_offset _targetoffset) -210.0 (* (`self.Step`) _targetoffset))) false true))
    (:`Finished`
      (set `self.Step` (+ (`self.Step`) 1)))))

(fn `UserConstructionScript`)