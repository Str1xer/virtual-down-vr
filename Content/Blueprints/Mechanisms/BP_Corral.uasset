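; Corral puzzle mechanism that is solved when a target number of BP_Enemy slimes are inside its box.
; Enemy begin and end overlaps recount the slimes, and CheckIsSolved reports whether the count matches the target.
; On a match during entry, a short delay precedes snapping the Gate to a hard-coded location and playing a timeline that pitches LinkedActor.
; Slimes leaving only update the count, without reversing either change.
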(event `self.Box.OnComponentBeginOverlap`
  (params (OverlappedComponent :type "PrimitiveComponent Object Reference") (OtherActor :type "Actor Object Reference") (OtherComp :type "PrimitiveComponent Object Reference") (OtherBodyIndex :type Integer) (bFromSweep :type Boolean) (SweepResult :type "HitResult Structure (by ref)"))
  (bind _linkedactor (`self.LinkedActor`))
  (bind (_returnvalue_roll _returnvalue_pitch _returnvalue_yaw) (`KismetMathLibrary.BreakRotator` (`self.K2_GetActorRotation` _linkedactor)))
  (if (== (`GameplayStatics.GetObjectClass` OtherActor) "/Game/Blueprints/Monsters/BP_Enemy.BP_Enemy_C")
    (bind _output_get (set `self.SlimeCount` (`KismetArrayLibrary.Array_Length` (`PrimitiveComponent.GetOverlappingActors` (`self.Box`) "/Game/Blueprints/Monsters/BP_Enemy.BP_Enemy_C"))))
    (`KismetSystemLibrary.PrintString` (`KismetStringLibrary.Conv_IntToString` _output_get))
    (if (== _output_get (`self.TargetCount`))
      (`KismetSystemLibrary.Delay` 0.3)
      (`self.K2_SetActorLocation` (`self.Gate`) (4705.768066 5103.924316 939.0) false false)
      (bind (_direction _rotation) (`Timeline|Start` :!via `PlayFromStart`)
        (:`Update`
          (`self.K2_SetActorRotation` _linkedactor (`KismetMathLibrary.MakeRotator` _returnvalue_roll _rotation _returnvalue_yaw) false))))))

(event `self.Box.OnComponentEndOverlap`
  (params (OverlappedComponent :type "PrimitiveComponent Object Reference") (OtherActor :type "Actor Object Reference") (OtherComp :type "PrimitiveComponent Object Reference") (OtherBodyIndex :type Integer))
  (if (== (`GameplayStatics.GetObjectClass` OtherActor) "/Game/Blueprints/Monsters/BP_Enemy.BP_Enemy_C")
    (set `self.SlimeCount` (`KismetArrayLibrary.Array_Length` (`PrimitiveComponent.GetOverlappingActors` (`self.Box`) "/Game/Blueprints/Monsters/BP_Enemy.BP_Enemy_C")))))

(fn `CheckIsSolved`
  (returns (State :type Boolean))
  (return (== (`self.SlimeCount`) (`self.TargetCount`))))

(fn `UserConstructionScript`)