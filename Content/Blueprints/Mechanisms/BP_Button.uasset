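; One-shot interactable button that sends an open message to a linked object when activated.
; Components tagged "Interaction" block a trace channel and show hover highlights through custom depth stencil values.
; Interacting sets it active, plays a sound, rotates the Sphere on a timeline, then disables highlight and trace blocking.
; CheckIsSolved exposes the active state.
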(event `self.ReceiveBeginPlay`
  (for _array_element (`self.GetComponentsByTag` "/Script/Engine.PrimitiveComponent" "Interaction")
    (`PrimitiveComponent.SetRenderCustomDepth` _array_element true)
    (`PrimitiveComponent.SetCollisionResponseToChannel` _array_element "ECC_GameTraceChannel3" "ECR_Block")))

(event `/Game/BPI_Interaction.Hover`
  (if (not (`self.Active`))
    (for _array_element (`self.GetComponentsByTag` "/Script/Engine.PrimitiveComponent" "Interaction")
      (`PrimitiveComponent.SetCustomDepthStencilValue` _array_element 1))))

(event `/Game/BPI_Interaction.Unhover`
  (for _array_element (`self.GetComponentsByTag` "/Script/Engine.PrimitiveComponent" "Interaction")
    (`PrimitiveComponent.SetCustomDepthStencilValue` _array_element 0)))

(event `/Game/BPI_Interaction.Interact`
  (params (Player :type "/Game/FirstPersonBP/Blueprints/BP__Player Object Reference"))
  (if (not (`self.Active`))
    (set `self.Active` true)
    (message `/Game/BPI_Door.Open` (`self.LinkedObject`))
    (`GameplayStatics.PlaySoundAtLocation` "/Game/Sounds/flashlight_on.flashlight_on" (`self.K2_GetActorLocation`) (struct) 1.0 1.0 0.0 null null null)
    (`self.RemoveInteractions`)
    (bind (_direction _newtrack_0) (`Timeline|Rotate` :!via `PlayFromStart`)
      (:`Update`
        (`SceneComponent.K2_SetRelativeRotation` (`self.Sphere`) (`KismetMathLibrary.MakeRotator` _newtrack_0) false false)))))

(fn `CheckIsSolved`
  (returns (State :type Boolean))
  (return (`self.Active`)))

(fn `RemoveInteractions`
  (for _array_element (`self.GetComponentsByTag` "/Script/Engine.PrimitiveComponent" "Interaction")
    (`PrimitiveComponent.SetCustomDepthStencilValue` _array_element 0)
    (`PrimitiveComponent.SetCollisionResponseToChannel` _array_element "ECC_GameTraceChannel3" "ECR_Overlap")))

(fn `UserConstructionScript`)