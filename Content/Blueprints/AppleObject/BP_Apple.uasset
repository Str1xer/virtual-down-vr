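; BP_Apple is a collectible apple that the player picks up through interaction.
; On BeginPlay, primitive components tagged "Interaction" enable custom depth rendering and block a custom trace channel (GameTraceChannel3).
; Hover and Unhover toggle those components' stencil value, presumably to drive a highlight effect.
; Interact increments the interacting player's ApplesCount and destroys the apple.
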(event `self.ReceiveBeginPlay`
  (for _array_element (`self.GetComponentsByTag` "/Script/Engine.PrimitiveComponent" "Interaction")
    (`PrimitiveComponent.SetRenderCustomDepth` _array_element true)
    (`PrimitiveComponent.SetCollisionResponseToChannel` _array_element "ECC_GameTraceChannel3" "ECR_Block")))

(event `/Game/BPI_Interaction.Hover`
  (for _array_element (`self.GetComponentsByTag` "/Script/Engine.PrimitiveComponent" "Interaction")
    (`PrimitiveComponent.SetCustomDepthStencilValue` _array_element 1)))

(event `/Game/BPI_Interaction.Unhover`
  (for _array_element (`self.GetComponentsByTag` "/Script/Engine.PrimitiveComponent" "Interaction")
    (`PrimitiveComponent.SetCustomDepthStencilValue` _array_element 0)))

(event `/Game/BPI_Interaction.Interact`
  (params (Player :type "/Game/FirstPersonBP/Blueprints/BP__Player Object Reference"))
  (set `/Game/FirstPersonBP/Blueprints/BP__Player.applesCount` (+ (`/Game/FirstPersonBP/Blueprints/BP__Player.applesCount` Player) 1) Player)
  (`self.K2_DestroyActor`))

(fn `UserConstructionScript`)