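; BP_Lever is a lever switch that opens a linked object and reports its on/off state through CheckIsSolved.
; A hit on Cube1 starts a looping timer, apparently for Checker, which reads the Sphere's roll.
; Negative roll activates it and sends OpenMessage once; otherwise it deactivates silently.
; The timer stops when rotation matches PrevRotation, but the node updating that variable is disconnected.
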(event `self.ReceiveBeginPlay`
  (`SceneComponent.K2_SetRelativeRotation` (`self.Sphere`) (struct :`Roll` 10.0) false false))

(event `self.Cube1.OnComponentHit`
  (params (HitComponent :type "PrimitiveComponent Object Reference") (OtherActor :type "Actor Object Reference") (OtherComp :type "PrimitiveComponent Object Reference") (NormalImpulse :type "Vector Structure") (Hit :type "HitResult Structure (by ref)"))
  (bind _returnvalue (`KismetSystemLibrary.K2_SetTimerDelegate` (`|CreateDelegate` :!event `Checker`) 0.1 true))
  (set `self.CheckerTimer` _returnvalue))

(fn `Checker`
  (if (== (`self.PrevRotation`) (`SceneComponent.RelativeRotation` (`self.Sphere`)))
    (`KismetSystemLibrary.K2_ClearAndInvalidateTimerHandle` (`self.CheckerTimer`))
    (elif (< (.roll (`SceneComponent.RelativeRotation` (`self.Sphere`))) 0.0)
      (if (not (`self.Active`))
        (set `self.Active` true)
        (message `/Game/BPI_Door.Open` (`self.LinkedObject`)))
      (elif (`self.Active`)
        (set `self.Active` false)))))

(fn `CheckIsSolved`
  (returns (State :type Boolean))
  (return (`self.Active`)))

(fn `UserConstructionScript`)