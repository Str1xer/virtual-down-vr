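; BP_Timer is an actor that counts elapsed seconds and shows the count on a TextRender component.
; StartTimer starts a looping one-second timer and stores its handle in TimerRef.
; Each tick increments Duration and passes it as text to UpdateText.
; Open clears the stored timer handle, stopping the count without resetting Duration.
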(event `UpdateText`
  (params (Value :type "Text (by ref)"))
  (`TextRenderComponent.K2_SetText` (`self.TextRender`) Value))

(event `/Game/BPI_Door.Open`
  (`KismetSystemLibrary.K2_ClearAndInvalidateTimerHandle` (`self.TimerRef`)))

(event `StartTimer`
  (bind _returnvalue (`KismetSystemLibrary.K2_SetTimerDelegate` (delegate `Timer`) 1.0 true))
  (set `self.TimerRef` _returnvalue))

(event `Timer`
  (bind _output_get (set `self.Duration` (+ (`self.Duration`) 1.0)))
  (`self.UpdateText` (`KismetTextLibrary.Conv_DoubleToText` _output_get "HalfToEven")))

(fn `UserConstructionScript`)