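; Actor component that runs a one-time dialogue sequence loaded from DT_Dialogues by DialogueKey.
; StartDialogue creates W_Dialogue, switches to UI-only input with a cursor, renders the first message and hides the player's inventory and navigation widgets.
; NextMessage and ReactOnResponse share identical logic: advance by one when NextId is 0, otherwise jump to that index.
; Past the end, they remove the widget, mark it Completed and restore game input and HUD.
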(event `StartDialogue`
  (bind _returnvalue (`GameplayStatics.GetPlayerController` 0))
  (if (not (`self.bCompleted`))
    (bind _returnvalue_2 (`|CreateWidget` "/Game/Blueprints/Dialogues/W_Dialogue.W_Dialogue_C" (`GameplayStatics.GetPlayerController` 0) self))
    (bind _output_get (set `self.Widget` _returnvalue_2))
    (`UserWidget.AddToViewport` _output_get 0)
    (`WidgetBlueprintLibrary.SetInputMode_UIOnlyEx` _returnvalue _output_get)
    (set `PlayerController.bShowMouseCursor` true _returnvalue)
    (bind _returnvalue_3 (`|GetDataTableRow` "/Game/Blueprints/Dialogues/DT_Dialogues.DT_Dialogues" (`self.DialogueKey`))
      (:`then`
        (set `self.CurrentIndex` 0)
        (bind _output_get_2 (set `self.DialogueSequence` (`.Sequence_3_F1563E1A4C74C150612DCFB4A6253AD2` (break `/Game/Blueprints/Dialogues/S_Dialogue` _returnvalue_3))))
        (`/Game/Blueprints/Dialogues/W_Dialogue.RenderMessage` (`self.Widget`) (`|GetArrayItem` _output_get_2 (`self.CurrentIndex`)))
        (bind _asbp__player (cast `/Game/FirstPersonBP/Blueprints/BP__Player` (`GameplayStatics.GetPlayerPawn` 0)))
        (`Widget.SetVisibility` (`/Game/FirstPersonBP/Blueprints/BP__Player.W_Inventory` _asbp__player) "Hidden")
        (`Widget.SetVisibility` (`/Game/FirstPersonBP/Blueprints/BP__Player.W_Navigations` _asbp__player) "Hidden")))))

(event `NextMessage`
  (params (NextId :type Integer))
  (bind _returnvalue (`GameplayStatics.GetPlayerController` 0))
  (set `self.CurrentIndex` (`KismetMathLibrary.SelectInt` (+ (`self.CurrentIndex`) 1) NextId (== NextId 0)))
  (if (< (`self.CurrentIndex`) (`KismetArrayLibrary.Array_Length` (`self.DialogueSequence`)))
    (`/Game/Blueprints/Dialogues/W_Dialogue.RenderMessage` (`self.Widget`) (`|GetArrayItem` (`self.DialogueSequence`) (`self.CurrentIndex`)))
    (else
      (`Widget.RemoveFromParent` (`self.Widget`))
      (set `self.bCompleted` true)
      (`WidgetBlueprintLibrary.SetInputMode_GameOnly` _returnvalue)
      (set `PlayerController.bShowMouseCursor` false _returnvalue)
      (bind _asbp__player (cast `/Game/FirstPersonBP/Blueprints/BP__Player` (`GameplayStatics.GetPlayerPawn` 0)))
      (`Widget.SetVisibility` (`/Game/FirstPersonBP/Blueprints/BP__Player.W_Inventory` _asbp__player) "SelfHitTestInvisible")
      (`Widget.SetVisibility` (`/Game/FirstPersonBP/Blueprints/BP__Player.W_Navigations` _asbp__player) "SelfHitTestInvisible"))))

(event `ReactOnResponse`
  (params (NextId :type Integer))
  (bind _returnvalue (`GameplayStatics.GetPlayerController` 0))
  (set `self.CurrentIndex` (`KismetMathLibrary.SelectInt` (+ (`self.CurrentIndex`) 1) NextId (== NextId 0)))
  (if (< (`self.CurrentIndex`) (`KismetArrayLibrary.Array_Length` (`self.DialogueSequence`)))
    (`/Game/Blueprints/Dialogues/W_Dialogue.RenderMessage` (`self.Widget`) (`|GetArrayItem` (`self.DialogueSequence`) (`self.CurrentIndex`)))
    (else
      (`Widget.RemoveFromParent` (`self.Widget`))
      (set `self.bCompleted` true)
      (`WidgetBlueprintLibrary.SetInputMode_GameOnly` _returnvalue)
      (set `PlayerController.bShowMouseCursor` false _returnvalue)
      (bind _asbp__player (cast `/Game/FirstPersonBP/Blueprints/BP__Player` (`GameplayStatics.GetPlayerPawn` 0)))
      (`Widget.SetVisibility` (`/Game/FirstPersonBP/Blueprints/BP__Player.W_Inventory` _asbp__player) "SelfHitTestInvisible")
      (`Widget.SetVisibility` (`/Game/FirstPersonBP/Blueprints/BP__Player.W_Navigations` _asbp__player) "SelfHitTestInvisible"))))