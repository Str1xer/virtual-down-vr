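; BP_VRApple is a grippable VR apple that tells the player character when it is held.
; Its grip and release events cast player pawn 0 to BP_VRCharacter and set or clear IsAppleInHand.
; The flag is a single boolean on the character, with no check of which hand or pawn did the gripping.
; Nodes that switch the static mesh's collision mode are present but unconnected, so they never run.
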(event `VRGripInterface.OnGrip`
  (params (GrippingController :type "GripMotionControllerComponent Object Reference") (GripInformation :type "BPActorGripInformation Structure (by ref)"))
  (bind _asbp_vrcharacter (cast `/Game/Blueprints/Character/BP_VRCharacter` (`GameplayStatics.GetPlayerPawn` 0)))
  (set `/Game/Blueprints/Character/BP_VRCharacter.bIsAppleInHand` true _asbp_vrcharacter))

(event `VRGripInterface.OnGripRelease`
  (params (ReleasingController :type "GripMotionControllerComponent Object Reference") (GripInformation :type "BPActorGripInformation Structure (by ref)") (bWasSocketed :type Boolean))
  (bind _asbp_vrcharacter (cast `/Game/Blueprints/Character/BP_VRCharacter` (`GameplayStatics.GetPlayerPawn` 0)))
  (set `/Game/Blueprints/Character/BP_VRCharacter.bIsAppleInHand` false _asbp_vrcharacter))

(fn `UserConstructionScript`)