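; Interactable robot NPC that starts dialogue on Interact and, with WithAnimation set, starts as loose physics parts that pull themselves together.
; After a delay, the parts stop simulating and attach to Mesh, then Tick interpolates them to hard-coded relative poses.
; A looping timer flip-flops a timeline to bob the Mesh vertically.
; "Interaction"-tagged components get custom-depth stencil hover highlighting and trace blocking, both removed once dialogue starts.
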(event `self.ReceiveBeginPlay`
  (bind _head (`self.head`))
  (`|ExecutionSequence`
    (:`then_0`
      (`KismetSystemLibrary.Delay` 5.0)
      (if (`self.bWithAnimation`)
        (`PrimitiveComponent.SetSimulatePhysics` (`self.body`) false)
        (`PrimitiveComponent.SetSimulatePhysics` (`self.head`) false)
        (`PrimitiveComponent.SetSimulatePhysics` (`self.hat`) false)
        (`PrimitiveComponent.SetSimulatePhysics` (`self.hands`) false)
        (`PrimitiveComponent.SetSimulatePhysics` (`self.hands1`) false)
        (`SceneComponent.K2_AttachToComponent` (`self.body`) (`self.Mesh`) "None" "KeepWorld" "KeepWorld" "KeepWorld" true)
        (`SceneComponent.K2_AttachToComponent` (`self.head`) (`self.Mesh`) "None" "KeepWorld" "KeepWorld" "KeepWorld" true)
        (`SceneComponent.K2_AttachToComponent` (`self.hat`) (`self.Mesh`) "None" "KeepWorld" "KeepWorld" "KeepWorld" true)
        (`SceneComponent.K2_AttachToComponent` (`self.hands`) (`self.Mesh`) "None" "KeepWorld" "KeepWorld" "KeepWorld" true)
        (`SceneComponent.K2_AttachToComponent` (`self.hands1`) (`self.Mesh`) "None" "KeepWorld" "KeepWorld" "KeepWorld" true)
        (set `self.bAnimationStarted` true))
      (for _array_element (`self.GetComponentsByTag` "/Script/Engine.PrimitiveComponent" "Interaction")
        (`PrimitiveComponent.SetRenderCustomDepth` _array_element true)
        (`PrimitiveComponent.SetCollisionResponseToChannel` _array_element "ECC_GameTraceChannel3" "ECR_Block")))
    (:`then_1`
      (`KismetSystemLibrary.K2_SetTimerDelegate` (delegate `Anim`) 2.0 true))
    (:`then_2`
      (`KismetSystemLibrary.Delay` 1.6)
      (if (`self.bWithAnimation`)
        (`GameplayStatics.PlaySoundAtLocation` "/Game/Sounds/falling-chandelier.falling-chandelier" (`self.K2_GetActorLocation`) (struct) 0.5 1.4 0.0 "/Game/Sounds/SlimeSplatConfig_2.SlimeSplatConfig_2" null null)))
    (:`then_3`
      (`GameplayStatics.SpawnSoundAttached` "/Game/Sounds/bank_00_instr_0036_snd_0000.bank_00_instr_0036_snd_0000" _head "None" (`SceneComponent.K2_GetComponentLocation` _head) (struct) "KeepRelativeOffset" false 1.0 1.2 0.0 "/Game/Sounds/WaaaConfig.WaaaConfig" null))))

(event `Anim`
  (`/Engine/EditorBlueprintResources/StandardMacros.FlipFlop`
    (:`A`
      (bind (_direction _newtrack_0) (`Timeline|UpDown` :!via `PlayFromStart` :!label _label)
        (:`Update`
          (`SceneComponent.K2_SetRelativeLocation` (`self.Mesh`) (`KismetMathLibrary.MakeVector` 0.0 0.0 (+ (* _newtrack_0 3.0) 30.0)) false false))))
    (:`B`
      (goto _label :!via `ReverseFromEnd`))))

(event `self.ReceiveTick`
  (params (DeltaSeconds :type "Float (single-precision)"))
  (if (`self.bAnimationStarted`)
    (`self.ReturnToTransform` (`self.body`) (0.0 0.0 -31.0) (struct :`Roll` -180.0) (0.3 0.3 0.3) DeltaSeconds)
    (`self.ReturnToTransform` (`self.head`) (0.0 0.0 0.0) (struct) (0.23 0.23 0.23) DeltaSeconds)
    (`self.ReturnToTransform` (`self.hat`) (0.0 0.0 16.0) (struct :`Roll` 180.0) (0.3 0.3 0.25) DeltaSeconds)
    (`self.ReturnToTransform` (`self.hands`) (0.0 32.0 -12.0) (struct :`Pitch` 9.5 :`Yaw` -11.5 :`Roll` 130.0) (0.08 0.08 0.08) DeltaSeconds)
    (`self.ReturnToTransform` (`self.hands1`) (0.0 -32.0 -12.0) (struct :`Pitch` 7.5 :`Yaw` 13.0 :`Roll` 240.0) (0.08 0.08 0.08) DeltaSeconds)))

(event `/Game/BPI_Interaction.Unhover`
  (for _array_element (`self.GetComponentsByTag` "/Script/Engine.PrimitiveComponent" "Interaction")
    (`PrimitiveComponent.SetCustomDepthStencilValue` _array_element 0)))

(event `/Game/BPI_Interaction.Hover`
  (if (not (`/Game/Blueprints/Dialogues/BP_DialogueComponent.bCompleted` (`self.BP_DialogueComponent`)))
    (for _array_element (`self.GetComponentsByTag` "/Script/Engine.PrimitiveComponent" "Interaction")
      (`PrimitiveComponent.SetCustomDepthStencilValue` _array_element 1))))

(event `/Game/BPI_Interaction.Interact`
  (params (Player :type "/Game/FirstPersonBP/Blueprints/BP__Player Object Reference"))
  (`/Game/Blueprints/Dialogues/BP_DialogueComponent.StartDialogue` (`self.BP_DialogueComponent`))
  (`self.RemoveInteractions`))

(fn `RemoveInteractions`
  (for _array_element (`self.GetComponentsByTag` "/Script/Engine.PrimitiveComponent" "Interaction")
    (`PrimitiveComponent.SetCustomDepthStencilValue` _array_element 0)
    (`PrimitiveComponent.SetCollisionResponseToChannel` _array_element "ECC_GameTraceChannel3" "ECR_Overlap")))

(fn `ReturnToTransform`
  (params (Target :type "SceneComponent Object Reference") (Location :type "Vector Structure") (Rotation :type "Rotator Structure") (Scale :type "Vector Structure") (DeltaTime :type "Float (double-precision)"))
  (`SceneComponent.K2_SetRelativeTransform` Target (`KismetMathLibrary.TInterpTo` (`SceneComponent.GetRelativeTransform` Target) (`KismetMathLibrary.MakeTransform` Location Rotation Scale) DeltaTime 5.0) true true))

(fn `UserConstructionScript`
  (set `/Game/Blueprints/Dialogues/BP_DialogueComponent.DialogueKey` (`self.DialogueName`) (`self.BP_DialogueComponent`))
  (`PrimitiveComponent.SetSimulatePhysics` (`self.body`) (`self.bWithAnimation`))
  (`PrimitiveComponent.SetSimulatePhysics` (`self.head`) (`self.bWithAnimation`))
  (`PrimitiveComponent.SetSimulatePhysics` (`self.hat`) (`self.bWithAnimation`))
  (`PrimitiveComponent.SetSimulatePhysics` (`self.hands`) (`self.bWithAnimation`))
  (`PrimitiveComponent.SetSimulatePhysics` (`self.hands1`) (`self.bWithAnimation`)))