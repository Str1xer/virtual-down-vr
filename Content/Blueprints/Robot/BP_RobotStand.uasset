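; BP_RobotStand is a robot stand actor made of body, head, hat and hand components, with physics simulation disabled on them at construction.
; ReturnToTransform eases a target component toward a given relative transform with TInterpTo, using sweep and teleport.
; RemoveInteractions clears the custom depth stencil on components tagged "Interaction" and sets their GameTraceChannel3 response to overlap.
; The event graph is empty, and neither helper is called within the file.
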(event `self.ReceiveBeginPlay`)

(event `Anim`)

(event `self.ReceiveTick`
  (params (DeltaSeconds :type "Float (single-precision)")))

(fn `RemoveInteractions`
  (for _array_element (`self.GetComponentsByTag` "/Script/Engine.PrimitiveComponent" "Interaction")
    (`PrimitiveComponent.SetCustomDepthStencilValue` _array_element 0)
    (`PrimitiveComponent.SetCollisionResponseToChannel` _array_element "ECC_GameTraceChannel3" "ECR_Overlap")))

(fn `ReturnToTransform`
  (params (Target :type "SceneComponent Object Reference") (Location :type "Vector Structure") (Rotation :type "Rotator Structure") (Scale :type "Vector Structure") (DeltaTime :type "Float (double-precision)"))
  (`SceneComponent.K2_SetRelativeTransform` Target (`KismetMathLibrary.TInterpTo` (`SceneComponent.GetRelativeTransform` Target) (`KismetMathLibrary.MakeTransform` Location Rotation Scale) DeltaTime 5.0) true true))

(fn `UserConstructionScript`
  (`PrimitiveComponent.SetSimulatePhysics` (`self.body`) false)
  (`PrimitiveComponent.SetSimulatePhysics` (`self.head`) false)
  (`PrimitiveComponent.SetSimulatePhysics` (`self.hat`) false)
  (`PrimitiveComponent.SetSimulatePhysics` (`self.hands`) false)
  (`PrimitiveComponent.SetSimulatePhysics` (`self.hands1`) false))