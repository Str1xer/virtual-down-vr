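; BP_CardObject is an interactable card pickup that gives the player cards and passes its Puzzle image to the player's Card.
; Construction applies the image through a dynamic material; components tagged Interaction get a trace channel block and custom-depth stencil toggled on hover.
; Interacting updates the player and destroys the actor.
; The WithFloat option adds a floating pickup hint and spawns BP_TriggerWithFloat at a hardcoded location after pickup, otherwise the widget is removed.
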(event `self.ReceiveBeginPlay`
  (if (`self.bWithFloat`)
    (bind _returnvalue (`|CreateWidget` "/Game/Widgets/Float/W_FLoat.W_Float_C" null "Возьмите карточку со стола"))
    (`WidgetComponent.SetWidget` (`self.Widget`) _returnvalue))
  (for _array_element (`self.GetComponentsByTag` "/Script/Engine.PrimitiveComponent" "Interaction")
    (`PrimitiveComponent.SetRenderCustomDepth` _array_element true)
    (`PrimitiveComponent.SetCollisionResponseToChannel` _array_element "ECC_GameTraceChannel3" "ECR_Block")))

(event `/Game/BPI_Interaction.Interact`
  (params (Player :type "/Game/FirstPersonBP/Blueprints/BP__Player Object Reference"))
  (set `/Game/FirstPersonBP/Blueprints/BP__Player.bHasCards` true Player)
  (`/Game/FirstPersonBP/Blueprints/A_Camera.ChangePuzzle` (`/Game/FirstPersonBP/Blueprints/BP__Player.Card` Player) (`self.Puzzle`))
  (`self.K2_DestroyActor`)
  (if (`self.bWithFloat`)
    (`|SpawnActorFromClass` "/Game/Tutorial/BP_TriggerWithFloat.BP_TriggerWithFloat_C" (`KismetMathLibrary.MakeTransform` (459.0 1090.0 206.0)) "Undefined" "OverrideRootScale" null null)))

(event `/Game/BPI_Interaction.Hover`
  (for _array_element (`self.GetComponentsByTag` "/Script/Engine.PrimitiveComponent" "Interaction")
    (`PrimitiveComponent.SetCustomDepthStencilValue` _array_element 1)))

(event `/Game/BPI_Interaction.Unhover`
  (for _array_element (`self.GetComponentsByTag` "/Script/Engine.PrimitiveComponent" "Interaction")
    (`PrimitiveComponent.SetCustomDepthStencilValue` _array_element 0)))

(fn `UserConstructionScript`
  (bind _returnvalue (`KismetMaterialLibrary.CreateDynamicMaterialInstance` "/Game/FirstPersonBP/Blueprints/M_CardObject.M_CardObject"))
  (`MaterialInstanceDynamic.SetTextureParameterValue` _returnvalue "Puzzle Image" (`self.Puzzle`))
  (`PrimitiveComponent.SetMaterial` (`self.Plane`) 0 _returnvalue)
  (if (not (`self.bWithFloat`))
    (`ActorComponent.K2_DestroyComponent` (`self.Widget`))))