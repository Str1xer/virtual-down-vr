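; BP_FinalButton is an interactable button that triggers the game's ending sequence.
; Components tagged "Interaction" render custom depth and block an interaction trace channel, with Hover and Unhover toggling their stencil value for highlighting.
; Interact switches possession to BP_EndCamera, reveals LinkedRobo, swaps all widgets for W_End and plays a final sound.
; It also runs the Move timeline, which drives LinkedObj's world Z position.
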(event `self.ReceiveBeginPlay`
  (for _array_element (`self.GetComponentsByTag` "/Script/Engine.PrimitiveComponent" "Interaction")
    (`PrimitiveComponent.SetRenderCustomDepth` _array_element true)
    (`PrimitiveComponent.SetCollisionResponseToChannel` _array_element "ECC_GameTraceChannel3" "ECR_Block")))

(event `/Game/BPI_Interaction.Hover`
  (for _array_element (`self.GetComponentsByTag` "/Script/Engine.PrimitiveComponent" "Interaction")
    (`PrimitiveComponent.SetCustomDepthStencilValue` _array_element 1)))

(event `/Game/BPI_Interaction.Unhover`
  (for _array_element (`self.GetComponentsByTag` "/Script/Engine.PrimitiveComponent" "Interaction")
    (`PrimitiveComponent.SetCustomDepthStencilValue` _array_element 0)))

(event `/Game/BPI_Interaction.Interact`
  (params (Player :type "/Game/FirstPersonBP/Blueprints/BP__Player Object Reference"))
  (bind _returnvalue (`GameplayStatics.GetPlayerController` 0))
  (bind _linkedobj (`self.LinkedObj`))
  (bind (_returnvalue_x _returnvalue_y) (`KismetMathLibrary.BreakVector` (`self.K2_GetActorLocation` _linkedobj)))
  (bind _returnvalue_2 (`GameplayStatics.GetActorOfClass` "/Game/BP_EndCamera.BP_EndCamera_C"))
  (`Controller.UnPossess` _returnvalue)
  (`Controller.Possess` _returnvalue _returnvalue_2)
  (`self.SetActorHiddenInGame` (`self.LinkedRobo`) false)
  (`WidgetLayoutLibrary.RemoveAllWidgets`)
  (bind _returnvalue_3 (`|CreateWidget` "/Game/Widgets/Menu/W_End.W_End_C"))
  (`UserWidget.AddToViewport` _returnvalue_3 0)
  (`GameplayStatics.PlaySoundAtLocation` "/Game/Sounds/rpreplay-final1612905681.rpreplay-final1612905681" (`self.K2_GetActorLocation`) (struct) 0.6 1.0 0.0 null null null)
  (bind (_direction _newtrack_0) (`Timeline|Move` :!via `PlayFromStart`)
    (:`Update`
      (`self.K2_SetActorLocation` _linkedobj (`KismetMathLibrary.MakeVector` _returnvalue_x _returnvalue_y _newtrack_0) false true))))

(fn `UserConstructionScript`)